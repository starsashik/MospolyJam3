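; MainCharacterBP is the player character Blueprint, and its only active logic is a horizontal dash in the DashBP event.
; The dash launches the character along the normalized current movement acceleration, or along the capsule's forward vector when acceleration is near zero.
; The launch zeroes the vertical component and adds to existing velocity rather than overriding it.
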(event EventBeginPlay)

(event EventDashBP
  (bind _charactermovement (Variables|Character|GetCharacterMovement))
  (bind _returnvalue (Pawn|Components|CharacterMovement|GetCurrentAcceleration _charactermovement))
  (bind _returnvalue_2 (Math|Vector|VectorLength _returnvalue))
  (if (< _returnvalue_2 0.01)
    (Character|LaunchCharacter (* (Math|Vector|GetForwardVector (Variables|Default|GetCapsuleComponent)) "1000.000000,1000.000000,0.000000") false false)
    (else
      (Character|LaunchCharacter (* (/ _returnvalue _returnvalue_2) "1000.000000,1000.000000,0.000000") false false))))

(fn ConstructionScript)