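; HUD Blueprint that tracks the screen center for a crosshair and holds a reference to the main character.
; Each DrawHUD call halves the viewport size and stores it as ScreenCenter; the graph itself draws nothing.
; It then casts player 0's pawn to MainCharacterBP only when the cached reference is invalid, so the lookup retries until it succeeds.
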(event EventDrawHUD
  (params (SizeX :type Integer) (SizeY :type Integer))
  ;[1 1 1] set screencenter for crosshair
  (Variables|Default|SetScreenCenter (Math|Vector2D|MakeVector2D (Math|Conversions|ToFloat(Integer) (/ SizeX 2)) (Math|Conversions|ToFloat(Integer) (/ SizeY 2))))
  (Utilities|IsValid (Variables|Default|GetAs%20Main%20Character%20BP)
    (:Is%20Not%20Valid
      (bind _asmain_character_bp (Utilities|Casting|CastToMainCharacterBP (Game|Player|GetPlayerPawn 0)))
      (Variables|Default|SetAs%20Main%20Character%20BP _asmain_character_bp))))

(fn ConstructionScript)