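; Door actor that slides open while either of its two ButtonForSitting child actors reports its condition as true.
; Each tick it reads both buttons and raises or lowers a clamped progress value, scaled by delta time.
; That value lerps the mesh between its BeginPlay location and an offset, reversing smoothly when both release.
; Audio starts once when the mesh leaves its start position and stops when it returns.
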(event EventBeginPlay
  (Variables|Default|SetInitial (Transformation|GetWorldLocation (Variables|Default|GetStaticMesh))))

(event EventTick
  (params (DeltaSeconds :type Float%20%28single-precision%29))
  (bind _delta (Variables|Default|GetDelta))
  (bind _tmetomove (Variables|Default|GetTmeToMove))
  (bind _staticmesh (Variables|Default|GetStaticMesh))
  (bind _initial (Variables|Default|GetInitial))
  (bind _returnvalue (+ _initial _delta))
  (Utilities|FlowControl|Sequence
    (:then_0
      (bind _asbutton_for_sitting (Utilities|Casting|CastToButtonForSitting (Variables|/Script/Engine.ChildActorComponent|GetChildActor (Variables|Default|GetButtonForSitting))))
      (Variables|Default|SetCond1 (Variables|/Game/Game/Blueprint/ButtonForSitting.ButtonForSitting_C|GetCondition _asbutton_for_sitting)))
    (:then_1
      (bind _asbutton_for_sitting_2 (Utilities|Casting|CastToButtonForSitting (Variables|/Script/Engine.ChildActorComponent|GetChildActor (Variables|Default|GetButtonForSitting1))))
      (Variables|Default|SetCond2 (Variables|/Game/Game/Blueprint/ButtonForSitting.ButtonForSitting_C|GetCondition _asbutton_for_sitting_2)))
    (:then_2
      (if (or (Variables|Default|GetCond1) (Variables|Default|GetCond2))
        (bind _output_get (Variables|Default|SetProgress (Math|Float|Clamp(Float) (+ (Variables|Default|GetProgress) (* DeltaSeconds _tmetomove)))))
        (Transformation|SetWorldLocation _staticmesh (Math|Vector|Lerp(Vector) _initial _returnvalue _output_get) false false)
        (else
          (bind _output_get_2 (Variables|Default|SetProgress (Math|Float|Clamp(Float) (- (Variables|Default|GetProgress) (* DeltaSeconds _tmetomove)))))
          (Transformation|SetWorldLocation _staticmesh (Math|Vector|Lerp(Vector) _initial _returnvalue _output_get_2) false false)))
      (if (>= (Math|Vector|VectorLength (Math|Vector|VectorGetAbs (- (Transformation|GetWorldLocation (Variables|Default|GetStaticMesh)) (Variables|Default|GetInitial)))) 2.0)
        (Utilities|FlowControl|DoOnce false :!label _label
          (:Completed
            (Audio|Components|Audio|Play (Variables|Default|GetAudio) 0.0)))
        (else
          (Audio|Components|Audio|Stop (Variables|Default|GetAudio))
          (goto _label Reset))))))

(fn ConstructionScript)