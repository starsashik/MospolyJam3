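; Display actor that shows a map's saved completion and collectable progress through glowing materials and a Niagara effect.
; On BeginPlay it creates dynamic material instances for a skeletal mesh and three wedge meshes, then loads MainSave.
; NumberMap selects the color and save entries: completion reveals Niagara and boosts cube power, while collectables light paired mesh materials.
; Maps 2 and 3 light some pairs unconditionally, having fewer collectable checks.
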(event EventBeginPlay
  (bind _niagara (Variables|Default|GetNiagara))
  (Utilities|FlowControl|Delay 0.05)
  (bind _returnvalue (Rendering|Material|CreateDynamicMaterialInstance "/Game/Game/Material/NonCube.NonCube" "None" "None" :!class /Script/Engine.KismetMaterialLibrary))
  (bind _output_get (Variables|Default|SetMat1 _returnvalue))
  (Rendering|Material|SetMaterial (Variables|Default|GetSkeletalMesh) 0 _output_get)
  (bind _returnvalue_2 (Rendering|Material|CreateDynamicMaterialInstance "/Game/Game/Material/NonCube.NonCube" "None" "None" :!class /Script/Engine.KismetMaterialLibrary))
  (bind _output_get_2 (Variables|Default|SetMat2 _returnvalue_2))
  (Rendering|Material|SetMaterial (Variables|Default|GetSkeletalMesh) 1 _output_get_2)
  (bind _returnvalue_3 (Rendering|Material|CreateDynamicMaterialInstance "/Game/Game/Material/NonCube.NonCube" "None" "None" :!class /Script/Engine.KismetMaterialLibrary))
  (bind _output_get_3 (Variables|Default|SetMat3 _returnvalue_3))
  (Rendering|Material|SetMaterial (Variables|Default|GetSkeletalMesh) 2 _output_get_3)
  (bind _returnvalue_4 (Rendering|Material|CreateDynamicMaterialInstance "/Game/Game/Material/NonCube.NonCube" "None" "None" :!class /Script/Engine.KismetMaterialLibrary))
  (bind _output_get_4 (Variables|Default|SetMat4 _returnvalue_4))
  (Rendering|Material|SetMaterial (Variables|Default|GetSkeletalMesh) 3 _output_get_4)
  (bind _returnvalue_5 (Rendering|Material|CreateDynamicMaterialInstance "/Game/Game/Material/ForCube.ForCube" "None" "None" :!class /Script/Engine.KismetMaterialLibrary))
  (bind _output_get_5 (Variables|Default|SetMat5 _returnvalue_5))
  (Rendering|Material|SetMaterial (Variables|Default|GetSkeletalMesh) 4 _output_get_5)
  (bind _returnvalue_6 (Rendering|Material|CreateDynamicMaterialInstance "/Game/Game/Material/ForCube_withFunc.ForCube_withFunc" "None" "None" :!class /Script/Engine.KismetMaterialLibrary))
  (bind _output_get_6 (Variables|Default|SetMat6 _returnvalue_6))
  (Rendering|Material|SetMaterial (Variables|Default|GetControlRig_Wedge_solid) 0 _output_get_6)
  (bind _returnvalue_7 (Rendering|Material|CreateDynamicMaterialInstance "/Game/Game/Material/ForCube_withFunc.ForCube_withFunc" "None" "None" :!class /Script/Engine.KismetMaterialLibrary))
  (bind _output_get_7 (Variables|Default|SetMat7 _returnvalue_7))
  (Rendering|Material|SetMaterial (Variables|Default|GetControlRig_Wedge_solid1) 0 _output_get_7)
  (bind _returnvalue_8 (Rendering|Material|CreateDynamicMaterialInstance "/Game/Game/Material/ForCube_withFunc.ForCube_withFunc" "None" "None" :!class /Script/Engine.KismetMaterialLibrary))
  (bind _output_get_8 (Variables|Default|SetMat8 _returnvalue_8))
  (Rendering|Material|SetMaterial (Variables|Default|GetControlRig_Wedge_solid2) 0 _output_get_8)
  (bind _returnvalue_9 (SaveGame|LoadGamefromSlot "MainSave"))
  (bind _asmy_main_save_game (Utilities|Casting|CastToMyMainSaveGame _returnvalue_9))
  (Variables|Default|SetCollectables (Variables|/Script/MyFPS.MyMainSaveGame|GetCollectables _asmy_main_save_game))
  (Rendering|Material|SetScalarParameterValue (Variables|Default|GetMat5) "Power" 2.0 :!class /Script/Engine.MaterialInstanceDynamic)
  (Rendering|Material|SetScalarParameterValue (Variables|Default|GetMat1) "Opacity" 0.5 :!class /Script/Engine.MaterialInstanceDynamic)
  (switch int (Variables|Default|GetNumberMap)
    (:Default
      (Development|PrintString "Выстави карту"))
    (:1
      (if (Variables|/Script/MyFPS.MyMainSaveGame|GetCompleteMap1 _asmy_main_save_game)
        (Rendering|SetVisibility _niagara true false)
        (Rendering|Material|SetScalarParameterValue (Variables|Default|GetMat5) "Power" 1e+02 :!class /Script/Engine.MaterialInstanceDynamic))
      (if (Utilities|Array|Get(acopy) (Variables|Default|GetCollectables))
        (Rendering|Material|SetScalarParameterValue (Variables|Default|GetMat2) "Opacity" 0.5 :!class /Script/Engine.MaterialInstanceDynamic)
        (Rendering|Material|SetScalarParameterValue (Variables|Default|GetMat6) "Power" 3e+01 :!class /Script/Engine.MaterialInstanceDynamic))
      (if (Utilities|Array|Get(acopy) (Variables|Default|GetCollectables) 1)
        (Rendering|Material|SetScalarParameterValue (Variables|Default|GetMat3) "Opacity" 0.5 :!class /Script/Engine.MaterialInstanceDynamic)
        (Rendering|Material|SetScalarParameterValue (Variables|Default|GetMat7) "Power" 3e+01 :!class /Script/Engine.MaterialInstanceDynamic))
      (if (Utilities|Array|Get(acopy) (Variables|Default|GetCollectables) 2)
        (Rendering|Material|SetScalarParameterValue (Variables|Default|GetMat4) "Opacity" 0.5 :!class /Script/Engine.MaterialInstanceDynamic)
        (Rendering|Material|SetScalarParameterValue (Variables|Default|GetMat8) "Power" 3e+01 :!class /Script/Engine.MaterialInstanceDynamic))
      (Rendering|Material|SetVectorParameterValue (Variables|Default|GetMat1) "Color" "(R=1.000000,G=0.364706,B=0.000000,A=1.000000)" :!class /Script/Engine.MaterialInstanceDynamic)
      (Rendering|Material|SetVectorParameterValue (Variables|Default|GetMat2) "Color" "(R=1.000000,G=0.364706,B=0.000000,A=1.000000)" :!class /Script/Engine.MaterialInstanceDynamic)
      (Rendering|Material|SetVectorParameterValue (Variables|Default|GetMat3) "Color" "(R=1.000000,G=0.364706,B=0.000000,A=1.000000)" :!class /Script/Engine.MaterialInstanceDynamic)
      (Rendering|Material|SetVectorParameterValue (Variables|Default|GetMat4) "Color" "(R=1.000000,G=0.364706,B=0.000000,A=1.000000)" :!class /Script/Engine.MaterialInstanceDynamic)
      (Rendering|Material|SetVectorParameterValue (Variables|Default|GetMat5) "Color" "(R=1.000000,G=0.364706,B=0.000000,A=1.000000)" :!class /Script/Engine.MaterialInstanceDynamic)
      (Rendering|Material|SetVectorParameterValue (Variables|Default|GetMat6) "Color" "(R=1.000000,G=0.364706,B=0.000000,A=1.000000)" :!class /Script/Engine.MaterialInstanceDynamic)
      (Rendering|Material|SetVectorParameterValue (Variables|Default|GetMat7) "Color" "(R=1.000000,G=0.364706,B=0.000000,A=1.000000)" :!class /Script/Engine.MaterialInstanceDynamic)
      (Rendering|Material|SetVectorParameterValue (Variables|Default|GetMat8) "Color" "(R=1.000000,G=0.364706,B=0.000000,A=1.000000)" :!class /Script/Engine.MaterialInstanceDynamic))
    (:2
      (if (Variables|/Script/MyFPS.MyMainSaveGame|GetCompleteMap2 _asmy_main_save_game)
        (Rendering|SetVisibility _niagara true false)
        (Rendering|Material|SetScalarParameterValue (Variables|Default|GetMat5) "Power" 1e+02 :!class /Script/Engine.MaterialInstanceDynamic))
      (if (Utilities|Array|Get(acopy) (Variables|Default|GetCollectables) 3)
        (Rendering|Material|SetScalarParameterValue (Variables|Default|GetMat2) "Opacity" 0.5 :!class /Script/Engine.MaterialInstanceDynamic)
        (Rendering|Material|SetScalarParameterValue (Variables|Default|GetMat6) "Power" 3e+01 :!class /Script/Engine.MaterialInstanceDynamic))
      (Rendering|Material|SetScalarParameterValue (Variables|Default|GetMat3) "Opacity" 0.5 :!class /Script/Engine.MaterialInstanceDynamic)
      (Rendering|Material|SetScalarParameterValue (Variables|Default|GetMat7) "Power" 3e+01 :!class /Script/Engine.MaterialInstanceDynamic)
      (if (Utilities|Array|Get(acopy) (Variables|Default|GetCollectables) 4)
        (Rendering|Material|SetScalarParameterValue (Variables|Default|GetMat4) "Opacity" 0.5 :!class /Script/Engine.MaterialInstanceDynamic)
        (Rendering|Material|SetScalarParameterValue (Variables|Default|GetMat8) "Power" 3e+01 :!class /Script/Engine.MaterialInstanceDynamic))
      (Rendering|Material|SetVectorParameterValue (Variables|Default|GetMat1) "Color" "(R=0.000000,G=0.894118,B=1.000000,A=1.000000)" :!class /Script/Engine.MaterialInstanceDynamic)
      (Rendering|Material|SetVectorParameterValue (Variables|Default|GetMat2) "Color" "(R=0.000000,G=0.894118,B=1.000000,A=1.000000)" :!class /Script/Engine.MaterialInstanceDynamic)
      (Rendering|Material|SetVectorParameterValue (Variables|Default|GetMat3) "Color" "(R=0.000000,G=0.894118,B=1.000000,A=1.000000)" :!class /Script/Engine.MaterialInstanceDynamic)
      (Rendering|Material|SetVectorParameterValue (Variables|Default|GetMat4) "Color" "(R=0.000000,G=0.894118,B=1.000000,A=1.000000)" :!class /Script/Engine.MaterialInstanceDynamic)
      (Rendering|Material|SetVectorParameterValue (Variables|Default|GetMat5) "Color" "(R=0.000000,G=0.894118,B=1.000000,A=1.000000)" :!class /Script/Engine.MaterialInstanceDynamic)
      (Rendering|Material|SetVectorParameterValue (Variables|Default|GetMat6) "Color" "(R=0.000000,G=0.894118,B=1.000000,A=1.000000)" :!class /Script/Engine.MaterialInstanceDynamic)
      (Rendering|Material|SetVectorParameterValue (Variables|Default|GetMat7) "Color" "(R=0.000000,G=0.894118,B=1.000000,A=1.000000)" :!class /Script/Engine.MaterialInstanceDynamic)
      (Rendering|Material|SetVectorParameterValue (Variables|Default|GetMat8) "Color" "(R=0.000000,G=0.894118,B=1.000000,A=1.000000)" :!class /Script/Engine.MaterialInstanceDynamic))
    (:3
      (if (Variables|/Script/MyFPS.MyMainSaveGame|GetCompleteMap3 _asmy_main_save_game)
        (Rendering|SetVisibility _niagara true false)
        (Rendering|Material|SetScalarParameterValue (Variables|Default|GetMat5) "Power" 1e+02 :!class /Script/Engine.MaterialInstanceDynamic))
      (Rendering|Material|SetScalarParameterValue (Variables|Default|GetMat2) "Opacity" 0.5 :!class /Script/Engine.MaterialInstanceDynamic)
      (Rendering|Material|SetScalarParameterValue (Variables|Default|GetMat6) "Power" 3e+01 :!class /Script/Engine.MaterialInstanceDynamic)
      (if (Utilities|Array|Get(acopy) (Variables|Default|GetCollectables) 5)
        (Rendering|Material|SetScalarParameterValue (Variables|Default|GetMat3) "Opacity" 0.5 :!class /Script/Engine.MaterialInstanceDynamic)
        (Rendering|Material|SetScalarParameterValue (Variables|Default|GetMat7) "Power" 3e+01 :!class /Script/Engine.MaterialInstanceDynamic))
      (Rendering|Material|SetScalarParameterValue (Variables|Default|GetMat4) "Opacity" 0.5 :!class /Script/Engine.MaterialInstanceDynamic)
      (Rendering|Material|SetScalarParameterValue (Variables|Default|GetMat8) "Power" 3e+01 :!class /Script/Engine.MaterialInstanceDynamic)
      (Rendering|Material|SetVectorParameterValue (Variables|Default|GetMat1) "Color" "(R=1.000000,G=0.000000,B=0.901961,A=1.000000)" :!class /Script/Engine.MaterialInstanceDynamic)
      (Rendering|Material|SetVectorParameterValue (Variables|Default|GetMat2) "Color" "(R=1.000000,G=0.000000,B=0.901961,A=1.000000)" :!class /Script/Engine.MaterialInstanceDynamic)
      (Rendering|Material|SetVectorParameterValue (Variables|Default|GetMat3) "Color" "(R=1.000000,G=0.000000,B=0.901961,A=1.000000)" :!class /Script/Engine.MaterialInstanceDynamic)
      (Rendering|Material|SetVectorParameterValue (Variables|Default|GetMat4) "Color" "(R=1.000000,G=0.000000,B=0.901961,A=1.000000)" :!class /Script/Engine.MaterialInstanceDynamic)
      (Rendering|Material|SetVectorParameterValue (Variables|Default|GetMat5) "Color" "(R=1.000000,G=0.000000,B=0.901961,A=1.000000)" :!class /Script/Engine.MaterialInstanceDynamic)
      (Rendering|Material|SetVectorParameterValue (Variables|Default|GetMat6) "Color" "(R=1.000000,G=0.000000,B=0.901961,A=1.000000)" :!class /Script/Engine.MaterialInstanceDynamic)
      (Rendering|Material|SetVectorParameterValue (Variables|Default|GetMat7) "Color" "(R=1.000000,G=0.000000,B=0.901961,A=1.000000)" :!class /Script/Engine.MaterialInstanceDynamic)
      (Rendering|Material|SetVectorParameterValue (Variables|Default|GetMat8) "Color" "(R=1.000000,G=0.000000,B=0.901961,A=1.000000)" :!class /Script/Engine.MaterialInstanceDynamic))))

(fn ConstructionScript)