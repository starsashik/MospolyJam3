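; Door actor that slides open while its child ButtonForSitting actor's Condition is true and slides back when false.
; Tick raises or lowers a clamped Progress by DeltaSeconds times TmeToMove (effectively a rate), lerping the mesh between its BeginPlay location and that location plus Delta.
; A DoOnce starts Audio once the mesh is displaced slightly, then stops and resets near the start position.
; Progress is printed every tick.
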(event EventBeginPlay
  (Variables|Default|SetInitial (Transformation|GetWorldLocation (Variables|Default|GetStaticMesh))))

(event Collision|EventActorBeginOverlap
  (params (OtherActor :type Actor%20Object%20Reference)))

(event EventTick
  (params (DeltaSeconds :type Float%20%28single-precision%29))
  (bind _staticmesh (Variables|Default|GetStaticMesh))
  (bind _delta (Variables|Default|GetDelta))
  (bind _tmetomove (Variables|Default|GetTmeToMove))
  (bind _initial (Variables|Default|GetInitial))
  (bind _returnvalue (+ _initial _delta))
  (bind _asbutton_for_sitting (Utilities|Casting|CastToButtonForSitting (Variables|/Script/Engine.ChildActorComponent|GetChildActor (Variables|Default|GetButtonForSitting))))
  (Development|PrintString (Utilities|String|ToString(Float) (Variables|Default|GetProgress)) true true "(R=0.000000,G=0.660000,B=1.000000,A=1.000000)" 0.0)
  (if (Variables|/Game/Game/Blueprint/ButtonForSitting.ButtonForSitting_C|GetCondition _asbutton_for_sitting)
    (bind _output_get (Variables|Default|SetProgress (Math|Float|Clamp(Float) (+ (Variables|Default|GetProgress) (* DeltaSeconds _tmetomove)))))
    (Transformation|SetWorldLocation _staticmesh (Math|Vector|Lerp(Vector) _initial _returnvalue _output_get) false false)
    (else
      (bind _output_get_2 (Variables|Default|SetProgress (Math|Float|Clamp(Float) (- (Variables|Default|GetProgress) (* DeltaSeconds _tmetomove)))))
      (Transformation|SetWorldLocation _staticmesh (Math|Vector|Lerp(Vector) _initial _returnvalue _output_get_2) false false)))
  (if (>= (Math|Vector|VectorLength (Math|Vector|VectorGetAbs (- (Transformation|GetWorldLocation (Variables|Default|GetStaticMesh)) (Variables|Default|GetInitial)))) 2.0)
    (Utilities|FlowControl|DoOnce false :!label _label
      (:Completed
        (Audio|Components|Audio|Play (Variables|Default|GetAudio) 0.0)))
    (else
      (Audio|Components|Audio|Stop (Variables|Default|GetAudio))
      (goto _label Reset))))

(fn ConstructionScript)