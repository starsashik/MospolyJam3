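; Collectable pickup actor, coloured by its ID through a dynamic material, that removes its mesh on start if the save already marks it collected.
; While its child-actor button's condition holds, Tick builds a timer and glow power while the mesh rises and jitters; releasing resets them.
; At the time threshold it plays a sound, removes the mesh, saves the collection, increments the player's count and calls StopSitting.
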(event EventBeginPlay
  (bind _returnvalue (Rendering|Material|CreateDynamicMaterialInstance "/Game/Game/Material/ForCube.ForCube" "None" "None" :!class /Script/Engine.KismetMaterialLibrary))
  (bind _output_get (Variables|Default|SetDynamicMat _returnvalue))
  (Rendering|Material|SetMaterial (Variables|Default|GetStaticMesh) 0 _output_get)
  (Utilities|FlowControl|Sequence
    (:then_0
      (Variables|Default|SetStartLoc (Transformation|GetWorldLocation (Variables|Default|GetStaticMesh)))
      (switch int (Variables|Default|GetIDCollectables)
        (:0
          (Variables|Default|SetColor "(R=1.000000,G=0.000000,B=0.124526,A=1.000000)"))
        (:1
          (Variables|Default|SetColor "(R=1.000000,G=0.000000,B=0.874342,A=1.000000)"))
        (:2
          (Variables|Default|SetColor "(R=0.000968,G=0.000000,B=1.000000,A=1.000000)"))
        (:3
          (Variables|Default|SetColor "(R=0.000000,G=0.967532,B=1.000000,A=1.000000)"))
        (:4
          (Variables|Default|SetColor "(R=0.000000,G=1.000000,B=0.182705,A=1.000000)"))
        (:5
          (Variables|Default|SetColor "(R=1.000000,G=0.934391,B=0.000000,A=1.000000)")))
      (Rendering|Material|SetVectorParameterValue (Variables|Default|GetDynamicMat) "Color" (Variables|Default|GetColor) :!class /Script/Engine.MaterialInstanceDynamic))
    (:then_1
      (Utilities|FlowControl|Delay 0.01)
      (bind _returnvalue_2 (SaveGame|LoadGamefromSlot "MainSave"))
      (bind _asmy_main_save_game (Utilities|Casting|CastToMyMainSaveGame _returnvalue_2))
      (if (Utilities|Array|Get(acopy) (Variables|/Script/MyFPS.MyMainSaveGame|GetCollectables _asmy_main_save_game) (Variables|Default|GetIDCollectables))
        (Components|DestroyComponent (Variables|Default|GetStaticMesh))
        (Variables|Default|SetCollect true)
        (Audio|Components|Audio|Stop (Variables|Default|GetAudio))))))

(event EventTick
  (params (DeltaSeconds :type Float%20%28single-precision%29))
  (if (not (Variables|Default|GetCollect))
    (bind _asbutton_for_collectables (Utilities|Casting|CastToButtonForCollectables (Variables|/Script/Engine.ChildActorComponent|GetChildActor (Variables|Default|GetButtonToCollectables))))
    (if (Variables|/Game/Game/Blueprint/ButtonForSitting.ButtonForSitting_C|GetCondition _asbutton_for_collectables)
      (bind _output_get (Variables|Default|SetTime (+ (Variables|Default|GetTime) DeltaSeconds)))
      (bind _output_get_2 (Variables|Default|SetPower (+ (Variables|Default|GetPower) (* DeltaSeconds 5e+01))))
      (Rendering|Material|SetScalarParameterValue (Variables|Default|GetDynamicMat) "Power" _output_get_2 :!class /Script/Engine.MaterialInstanceDynamic)
      (Transformation|AddWorldOffset (Variables|Default|GetStaticMesh) (Math|Vector|MakeVector (Math|Random|RandomFloatinRange -3.0 3.0) (Math|Random|RandomFloatinRange -3.0 3.0) (* DeltaSeconds 2e+01)) false false)
      (if (>= _output_get (Variables|Default|GetTimeToCollect))
        (Development|PrintString "VFX for Collectables")
        (Audio|PlaySoundatLocation "/Game/Game/Sound_Logic/Sounds/CollectCollectables.CollectCollectables" (Transformation|GetWorldLocation (Variables|Default|GetStaticMesh)) "0, 0, 0" 1.0 1.0 0.0 0 0 0 0)
        (Components|DestroyComponent (Variables|Default|GetStaticMesh))
        (Variables|Default|SetCollect true)
        (bind _returnvalue (SaveGame|LoadGamefromSlot "MainSave"))
        (bind _asmy_main_save_game (Utilities|Casting|CastToMyMainSaveGame _returnvalue))
        (Utilities|Array|SetArrayElem (Variables|/Script/MyFPS.MyMainSaveGame|GetCollectables _asmy_main_save_game) (Variables|Default|GetIDCollectables) true)
        (SaveGame|SaveGametoSlot _asmy_main_save_game "MainSave")
        (Audio|Components|Audio|Stop (Variables|Default|GetAudio))
        (bind _asmain_character_bp (Utilities|Casting|CastToMainCharacterBP (Game|Player|GetPlayerPawn 0)))
        (Variables|/Game/Game/Player/MainCharacterBP.MainCharacterBP_C|SetCurrentCollect _asmain_character_bp (+ (Variables|/Game/Game/Player/MainCharacterBP.MainCharacterBP_C|GetCurrentCollect _asmain_character_bp) 1))
        (Class|MainCharacter|StopSitting _asmain_character_bp))
      (else
        (Variables|Default|SetTime 0.0)
        (Transformation|SetWorldLocation (Variables|Default|GetStaticMesh) (Variables|Default|GetStartLoc) false false)
        (bind _output_get_3 (Variables|Default|SetPower 2.0))
        (Rendering|Material|SetScalarParameterValue (Variables|Default|GetDynamicMat) "Power" _output_get_3 :!class /Script/Engine.MaterialInstanceDynamic)))))

(fn ConstructionScript)