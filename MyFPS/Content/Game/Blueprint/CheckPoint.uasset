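; Checkpoint actor that saves player progress and lets the player travel to FirstPersonMap.
; When MainCharacterBP overlaps its box, it writes its checkpoint ID to the MainSave slot field for its map number, sets CurrentMap to 0 and plays an activation sound.
; Tick times how long the child ButtonForSitting's condition holds, resetting otherwise, and opens FirstPersonMap through ROPGameInstance once TimeToInteract is reached.
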(event OnComponentBeginOverlap(Box)
  (params (OverlappedComponent :type Primitive%20Component%20Object%20Reference) (OtherActor :type Actor%20Object%20Reference) (OtherComp :type Primitive%20Component%20Object%20Reference) (OtherBodyIndex :type Integer) (bFromSweep :type Boolean) (SweepResult :type Hit%20Result%20Structure%20%28by%20ref%29))
  (bind _idcheckpoint (Variables|Default|GetidCheckPoint))
  (Utilities|Casting|CastToMainCharacterBP OtherActor)
  (bind _returnvalue (SaveGame|LoadGamefromSlot "MainSave"))
  (bind _asmy_main_save_game (Utilities|Casting|CastToMyMainSaveGame _returnvalue))
  (switch int (Variables|Default|GetNumerMap)
    (:Default
      (Development|PrintString "Выстави номер мира"))
    (:1
      (Variables|/Script/MyFPS.MyMainSaveGame|SetIdCheckPointMap1 _asmy_main_save_game _idcheckpoint)
      (Variables|/Script/MyFPS.MyMainSaveGame|SetCurrentMap _asmy_main_save_game 0 :!label _label)
      (SaveGame|SaveGametoSlot _asmy_main_save_game "MainSave")
      (Audio|PlaySoundatLocation "/Game/Game/Sound_Logic/Sounds/ActivateCheckPoint.ActivateCheckPoint" (Transformation|GetWorldLocation (Variables|Default|GetBox)) "0, 0, 0" 1.0 1.0 0.0 0 0 0 0))
    (:2
      (Variables|/Script/MyFPS.MyMainSaveGame|SetIdCheckPointMap2 _asmy_main_save_game _idcheckpoint)
      (goto _label))
    (:3
      (Variables|/Script/MyFPS.MyMainSaveGame|SetIdCheckPointMap3 _asmy_main_save_game _idcheckpoint)
      (goto _label))))

(event EventTick
  (params (DeltaSeconds :type Float%20%28single-precision%29))
  (bind _asbutton_for_sitting (Utilities|Casting|CastToButtonForSitting (Variables|/Script/Engine.ChildActorComponent|GetChildActor (Variables|Default|GetButtonForSitting))))
  (if (Variables|/Game/Game/Blueprint/ButtonForSitting.ButtonForSitting_C|GetCondition _asbutton_for_sitting)
    (bind _output_get (Variables|Default|SetTime (+ (Variables|Default|GetTime) DeltaSeconds)))
    (if (>= _output_get (Variables|Default|GetTimeToInteract))
      (bind _asropgame_instance (Utilities|Casting|CastToROPGameInstance (Game|GetGameInstance)))
      (Default|OpenMyLevels _asropgame_instance "" "/Game/FirstPerson/Maps/FirstPersonMap.FirstPersonMap"))
    (else
      (Variables|Default|SetTime 0.0))))

(fn ConstructionScript)