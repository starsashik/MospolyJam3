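; Moving platform actor whose skeletal mesh shuttles endlessly between two marker components, CubeA and CubeB.
; On BeginPlay it teleports the mesh to CubeA, then loops eased MoveComponentTo moves to CubeB and back, matching each cube's relative rotation with a small Z offset.
; TimeToMove sets each leg's duration, and a short delay follows each return to CubeA before the cycle repeats.
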(event EventBeginPlay
  (bind _skeletalmesh (Variables|Default|GetSkeletalMesh))
  (bind _cubea (Variables|Default|GetCubeA))
  (bind _cubeb (Variables|Default|GetCubeB))
  (bind _timetomove (Variables|Default|GetTimeToMove))
  (bind _relativelocation (Variables|/Script/Engine.SceneComponent|GetRelativeLocation _cubea))
  (bind _relativelocation_2 (Variables|/Script/Engine.SceneComponent|GetRelativeLocation _cubeb))
  (Transformation|SetRelativeLocation _skeletalmesh (Variables|/Script/Engine.SceneComponent|GetRelativeLocation (Variables|Default|GetCubeA)) false true)
  (Components|MoveComponentTo _skeletalmesh (Math|Vector|MakeVector (.x _relativelocation_2) (.y _relativelocation_2) (+ (.z _relativelocation_2) 15.0)) (Variables|/Script/Engine.SceneComponent|GetRelativeRotation _cubeb) true true _timetomove false :!label _label)
  (Components|MoveComponentTo _skeletalmesh (Math|Vector|MakeVector (.x _relativelocation) (.y _relativelocation) (+ (.z _relativelocation) 15.0)) (Variables|/Script/Engine.SceneComponent|GetRelativeRotation _cubea) true true _timetomove false)
  (Utilities|FlowControl|Delay 1.0)
  (goto _label))

(fn ConstructionScript)