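; Level transition actor that sends the game to level Mir1 after a child ButtonForSitting stays active for a set time.
; Tick accumulates time while the button's condition holds, resets it otherwise, then writes the player's location to the MainSave slot and opens the level through ROPGameInstance.
; BeginPlay caches the three map-completion flags from the save and gives the map and in/out cubes separate dynamic materials.
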(event EventBeginPlay
  (bind _returnvalue (SaveGame|LoadGamefromSlot "MainSave"))
  (bind _asmy_main_save_game (Utilities|Casting|CastToMyMainSaveGame _returnvalue)
    (:then
      (Variables|Default|SetComplete%20Map%201 (Variables|/Script/MyFPS.MyMainSaveGame|GetCompleteMap1 _asmy_main_save_game))
      (Variables|Default|SetComplete%20Map%202 (Variables|/Script/MyFPS.MyMainSaveGame|GetCompleteMap2 _asmy_main_save_game))
      (Variables|Default|SetComplete%20Map%203 (Variables|/Script/MyFPS.MyMainSaveGame|GetCompleteMap3 _asmy_main_save_game)))
    (:CastFailed
      _))
  (bind _returnvalue_2 (Rendering|Material|CreateDynamicMaterialInstance "/Game/Game/Material/ForCube.ForCube" "None" "None" :!class /Script/Engine.KismetMaterialLibrary))
  (bind _output_get (Variables|Default|SetMat1 _returnvalue_2))
  (Rendering|Material|SetMaterial (Variables|Default|GetMap1) 0 _output_get)
  (bind _returnvalue_3 (Rendering|Material|CreateDynamicMaterialInstance "/Game/Game/Material/ForCube.ForCube" "None" "None" :!class /Script/Engine.KismetMaterialLibrary))
  (bind _output_get_2 (Variables|Default|SetMat2 _returnvalue_3))
  (Rendering|Material|SetMaterial (Variables|Default|GetMap2) 0 _output_get_2)
  (bind _returnvalue_4 (Rendering|Material|CreateDynamicMaterialInstance "/Game/Game/Material/ForCube.ForCube" "None" "None" :!class /Script/Engine.KismetMaterialLibrary))
  (bind _output_get_3 (Variables|Default|SetMat3 _returnvalue_4))
  (Rendering|Material|SetMaterial (Variables|Default|GetMap3) 0 _output_get_3)
  (bind _returnvalue_5 (Rendering|Material|CreateDynamicMaterialInstance "/Game/Game/Material/ForCube.ForCube" "None" "None" :!class /Script/Engine.KismetMaterialLibrary))
  (bind _output_get_4 (Variables|Default|SetOut _returnvalue_5))
  (Rendering|Material|SetMaterial (Variables|Default|GetCubeOut) 0 _output_get_4)
  (bind _returnvalue_6 (Rendering|Material|CreateDynamicMaterialInstance "/Game/Game/Material/ForCube.ForCube" "None" "None" :!class /Script/Engine.KismetMaterialLibrary))
  (bind _output_get_5 (Variables|Default|SetIn _returnvalue_6))
  (Rendering|Material|SetMaterial (Variables|Default|GetCubeIn) 0 _output_get_5))

(event EventTick
  (params (DeltaSeconds :type Float%20%28single-precision%29))
  (Utilities|FlowControl|Sequence
    (:then_0
      (if true
        (bind _asbutton_for_sitting (Utilities|Casting|CastToButtonForSitting (Variables|/Script/Engine.ChildActorComponent|GetChildActor (Variables|Default|GetButtonForSitting))))
        (if (Variables|/Game/Game/Blueprint/ButtonForSitting.ButtonForSitting_C|GetCondition _asbutton_for_sitting)
          (bind _output_get (Variables|Default|SetTime (+ (Variables|Default|GetTime) DeltaSeconds)))
          (if (>= _output_get (Variables|Default|GetTimeToInteractPereh))
            (Variables|Default|SetTime 0.0)
            (bind _asmain_character_bp (Utilities|Casting|CastToMainCharacterBP (Game|Player|GetPlayerPawn 0)))
            (bind _returnvalue (SaveGame|LoadGamefromSlot "MainSave"))
            (bind _asmy_main_save_game (Utilities|Casting|CastToMyMainSaveGame _returnvalue))
            (Variables|/Script/MyFPS.MyMainSaveGame|SetPlayerLoc _asmy_main_save_game (Transformation|GetActorLocation _asmain_character_bp))
            (SaveGame|SaveGametoSlot _asmy_main_save_game "MainSave")
            (if true
              (bind _asropgame_instance (Utilities|Casting|CastToROPGameInstance (Game|GetGameInstance)))
              (Default|OpenMyLevels _asropgame_instance "" "/Game/Game/Maps/Mir1.Mir1")))
          (else
            (Variables|Default|SetTime 0.0)))))))

(fn ConstructionScript)