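; Finish trigger actor that ends the game with a cutscene once the player has earned it.
; On BeginPlay it reads the MainSave slot, counts collected items and destroys itself unless all six are set.
; When the main character enters its box, it hides once, mutes music and sound classes via sound mix overrides, and plays the Finish level sequence.
; After a fixed delay it opens the start map.
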(event OnComponentBeginOverlap(Box)
  (params (OverlappedComponent :type Primitive%20Component%20Object%20Reference) (OtherActor :type Actor%20Object%20Reference) (OtherComp :type Primitive%20Component%20Object%20Reference) (OtherBodyIndex :type Integer) (bFromSweep :type Boolean) (SweepResult :type Hit%20Result%20Structure%20%28by%20ref%29))
  (bind _asmain_character_bp (Utilities|Casting|CastToMainCharacterBP OtherActor))
  (Variables|Default|SetAs%20Main%20Character%20BP _asmain_character_bp)
  (Utilities|FlowControl|DoOnce false
    (:Completed
      (Rendering|SetActorHiddenInGame true)
      (Audio|SetSoundMixClassOverride "/Game/Game/Sound_Logic/SoundClassMix.SoundClassMix" "/Game/Game/Sound_Logic/MusicSoundClass.MusicSoundClass" 0.0 1.0 0.0 true)
      (Audio|SetSoundMixClassOverride "/Game/Game/Sound_Logic/SoundClassMix.SoundClassMix" "/Game/Game/Sound_Logic/SoundClass.SoundClass" 0.0 1.0 0.0 true)
      (bind _returnvalue (Sequencer|Player|CreateLevelSequencePlayer "/Game/Game/Cinematic/Finish.Finish" (Utilities|Struct|MakeMovieSceneSequencePlaybackSettings false "(Value=0)" 1.0 0.0 false false true true true true false true)))
      (Sequencer|Player|Play _returnvalue :!class /Script/MovieScene.MovieSceneSequencePlayer)
      (Utilities|FlowControl|Delay 11.0)
      (Game|OpenLevel(byObjectReference) "/Game/Game/Maps/StartMap.StartMap"))))

(event EventBeginPlay
  (bind _returnvalue (SaveGame|LoadGamefromSlot "MainSave"))
  (bind _asmy_main_save_game (Utilities|Casting|CastToMyMainSaveGame _returnvalue))
  (for _array_element (Variables|/Script/MyFPS.MyMainSaveGame|GetCollectables _asmy_main_save_game)
    (if _array_element
      (Variables|Default|Setproverka (+ (Variables|Default|Getproverka) 1))))
  (if (not (== (Variables|Default|Getproverka) 6))
    (Actor|DestroyActor)))

(event Collision|EventActorBeginOverlap
  (params (OtherActor :type Actor%20Object%20Reference)))

(event EventTick
  (params (DeltaSeconds :type Float%20%28single-precision%29)))

(fn ConstructionScript)