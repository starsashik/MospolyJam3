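; A button actor that activates when the main character sits inside its trigger box.
; Box overlaps cache the character and toggle a prompt widget.
; Tick polls the character's sitting state and, through a DoOnce, plays the activation animation and audio and sets a Condition flag.
; Standing up or leaving the box clears the flag, stops the audio and resets the DoOnce.
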(event OnComponentBeginOverlap(Box)
  (params (OverlappedComponent :type Primitive%20Component%20Object%20Reference) (OtherActor :type Actor%20Object%20Reference) (OtherComp :type Primitive%20Component%20Object%20Reference) (OtherBodyIndex :type Integer) (bFromSweep :type Boolean) (SweepResult :type Hit%20Result%20Structure%20%28by%20ref%29))
  (bind _asmain_character_bp (Utilities|Casting|CastToMainCharacterBP OtherActor))
  (Variables|Default|SetAs%20Main%20Character%20BP _asmain_character_bp)
  (Variables|Default|SetPlayer? true)
  (Rendering|SetVisibility (Variables|Default|GetWidget) true false))

(event OnComponentEndOverlap(Box)
  (params (OverlappedComponent :type Primitive%20Component%20Object%20Reference) (OtherActor :type Actor%20Object%20Reference) (OtherComp :type Primitive%20Component%20Object%20Reference) (OtherBodyIndex :type Integer))
  (Utilities|Casting|CastToMainCharacterBP OtherActor)
  (Variables|Default|SetAs%20Main%20Character%20BP 0)
  (Variables|Default|SetPlayer? false)
  (Rendering|SetVisibility (Variables|Default|GetWidget) false false))

(event EventTick
  (params (DeltaSeconds :type Float%20%28single-precision%29))
  (if (Variables|Default|GetPlayer?)
    (if (Class|MainCharacter|GetSitting (Variables|Default|GetAs%20Main%20Character%20BP))
      (Utilities|FlowControl|DoOnce false :!label _label
        (:Completed
          (Components|Animation|PlayAnimation (Variables|Default|GetSkeletalMesh) 0 false)
          (Variables|Default|SetCondition true)
          (Development|PrintString "Hello" true true "(R=0.000000,G=0.660000,B=1.000000,A=1.000000)" 1.0)
          (Audio|Components|Audio|Play (Variables|Default|GetAudio) 0.0)
          (Components|Animation|PlayAnimation (Variables|Default|GetSkeletalMesh) "/Game/Game/Models/Button/Button_Anim_SK_Button_Activate.Button_Anim_SK_Button_Activate" false)))
      (else
        (Variables|Default|SetCondition false :!label _label_2)
        (Audio|Components|Audio|Stop (Variables|Default|GetAudio))
        (goto _label Reset)))
    (else
      (goto _label_2))))

(fn ConstructionScript)