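; Display stand that shows whether the collectable matching its ID has been collected.
; On BeginPlay it reads the MainSave slot after a short delay; if collected, it plays audio and sets a diamond mesh with a dynamic material colored per ID (six colors).
; Once active, Tick flickers the material's Power randomly and moves the mesh with clamped X/Y jitter while raising it to a height limit.
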(event EventBeginPlay
  (bind _returnvalue (Rendering|Material|CreateDynamicMaterialInstance "/Game/Game/Material/ForCube.ForCube" "None" "None" :!class /Script/Engine.KismetMaterialLibrary))
  (Variables|Default|SetDynamicMat _returnvalue)
  (Utilities|FlowControl|Delay 0.01)
  (bind _returnvalue_2 (SaveGame|LoadGamefromSlot "MainSave"))
  (bind _asmy_main_save_game (Utilities|Casting|CastToMyMainSaveGame _returnvalue_2))
  (if (Utilities|Array|Get(acopy) (Variables|/Script/MyFPS.MyMainSaveGame|GetCollectables _asmy_main_save_game) (Variables|Default|GetIDCollectables))
    (switch int (Variables|Default|GetIDCollectables)
      (:0
        (Variables|Default|SetColor "(R=1.000000,G=0.000000,B=0.124526,A=1.000000)"))
      (:1
        (Variables|Default|SetColor "(R=1.000000,G=0.000000,B=0.874342,A=1.000000)"))
      (:2
        (Variables|Default|SetColor "(R=0.000968,G=0.000000,B=1.000000,A=1.000000)"))
      (:3
        (Variables|Default|SetColor "(R=0.000000,G=0.967532,B=1.000000,A=1.000000)"))
      (:4
        (Variables|Default|SetColor "(R=0.000000,G=1.000000,B=0.182705,A=1.000000)"))
      (:5
        (Variables|Default|SetColor "(R=1.000000,G=0.934391,B=0.000000,A=1.000000)")))
    (Rendering|Material|SetVectorParameterValue (Variables|Default|GetDynamicMat) "Color" (Variables|Default|GetColor) :!class /Script/Engine.MaterialInstanceDynamic)
    (Variables|Default|SetCollect true)
    (Audio|Components|Audio|Play (Variables|Default|GetAudio) 0.0)
    (Components|StaticMesh|SetStaticMesh (Variables|Default|GetStaticMesh) "/ControlRig/Controls/ControlRig_Diamond_solid.ControlRig_Diamond_solid")
    (Rendering|Material|SetMaterial (Variables|Default|GetStaticMesh) 0 (Variables|Default|GetDynamicMat))))

(event EventTick
  (params (DeltaSeconds :type Float%20%28single-precision%29))
  (bind _staticmesh (Variables|Default|GetStaticMesh))
  (bind _relativelocation (Variables|/Script/Engine.SceneComponent|GetRelativeLocation _staticmesh))
  (if (Variables|Default|GetCollect)
    (Rendering|Material|SetScalarParameterValue (Variables|Default|GetDynamicMat) "Power" (Math|Random|RandomFloatinRange 25.0 1e+02) :!class /Script/Engine.MaterialInstanceDynamic)
    (Transformation|SetRelativeLocation (Variables|Default|GetStaticMesh) (Math|Vector|MakeVector (Math|Float|Clamp(Float) (+ (.x _relativelocation) (Math|Random|RandomFloatinRange -1.0 1.0)) -3e+01 3e+01) (Math|Float|Clamp(Float) (+ (.y _relativelocation) (Math|Random|RandomFloatinRange -1.0 1.0)) -3e+01 3e+01) (Math|Float|Clamp(Float) (+ (.z _relativelocation) (Math|Random|RandomFloatinRange 3.0 3.0)) 7e+01 1.3e+02)) false false)))

(fn ConstructionScript)