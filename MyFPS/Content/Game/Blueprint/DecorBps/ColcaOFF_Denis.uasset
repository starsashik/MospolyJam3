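; Decorative actor that continuously spins three components, Colso1 to Colso3, which appear to be rings.
; Every Tick adds a local pitch rotation to each, scaled by delta time for frame-rate-independent motion.
; The first two turn in opposite directions at equal speed, while the third turns at half that speed.
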(event EventBeginPlay)

(event Collision|EventActorBeginOverlap
  (params (OtherActor :type Actor%20Object%20Reference)))

(event EventTick
  (params (DeltaSeconds :type Float%20%28single-precision%29))
  (Transformation|AddLocalRotation (Variables|Default|GetColso1) (Math|Rotator|MakeRotator 0.0 (* DeltaSeconds 1e+01) 0.0) false false)
  (Transformation|AddLocalRotation (Variables|Default|GetColso2) (Math|Rotator|MakeRotator 0.0 (* DeltaSeconds -1e+01) 0.0) false false)
  (Transformation|AddLocalRotation (Variables|Default|GetColso3) (Math|Rotator|MakeRotator 0.0 (* DeltaSeconds 5.0) 0.0) false false))

(fn ConstructionScript)