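; EndMir is a lever actor that marks one of three worlds, chosen by its Mir number, as complete.
; On BeginPlay it reads the MainSave slot and swings the lever to its activated rotation if that world is already completed.
; Otherwise Tick polls a child ButtonForCollectables until its condition and hold time are met.
; It then calls StopSitting on the player, rotates the lever, saves the completion flag and plays a sound.
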(event EventBeginPlay
  (bind _returnvalue (SaveGame|LoadGamefromSlot "MainSave"))
  (bind _asmy_main_save_game (Utilities|Casting|CastToMyMainSaveGame _returnvalue))
  (switch int (Variables|Default|GetMir)
    (:1
      (if (Variables|/Script/MyFPS.MyMainSaveGame|GetCompleteMap1 _asmy_main_save_game)
        (Variables|Default|SetCondition true :!label _label)
        (Components|MoveComponentTo (Variables|Default|GetLever) "0, 0, 0" "-40.000000,0.000000,0.000000" true true 3.0 true)))
    (:2
      (if (Variables|/Script/MyFPS.MyMainSaveGame|GetCompleteMap2 _asmy_main_save_game)
        (goto _label)))
    (:3
      (if (Variables|/Script/MyFPS.MyMainSaveGame|GetCompleteMap3 _asmy_main_save_game)
        (goto _label)))))

(event EventTick
  (params (DeltaSeconds :type Float%20%28single-precision%29))
  (if (not (Variables|Default|GetCondition))
    (bind _asbutton_for_collectables (Utilities|Casting|CastToButtonForCollectables (Variables|/Script/Engine.ChildActorComponent|GetChildActor (Variables|Default|GetButtonForCollectables))))
    (if (Variables|/Game/Game/Blueprint/ButtonForSitting.ButtonForSitting_C|GetCondition _asbutton_for_collectables)
      (if (>= (Variables|/Game/Game/Blueprint/ButtonForSitting.ButtonForSitting_C|GetTime _asbutton_for_collectables) (Variables|Default|GetTime%20to%20Interact%20))
        (bind _asmain_character_bp (Utilities|Casting|CastToMainCharacterBP (Game|Player|GetPlayerPawn 0)))
        (Class|MainCharacter|StopSitting _asmain_character_bp)
        (Variables|Default|SetCondition true)
        (Components|MoveComponentTo (Variables|Default|GetLever) "0, 0, 0" "-40.000000,0.000000,0.000000" true true 3.0 true)
        (bind _returnvalue (SaveGame|LoadGamefromSlot "MainSave"))
        (bind _asmy_main_save_game (Utilities|Casting|CastToMyMainSaveGame _returnvalue))
        (switch int (Variables|Default|GetMir)
          (:Default
            (Development|PrintString "Задай номер мира"))
          (:1
            (Variables|/Script/MyFPS.MyMainSaveGame|SetCompleteMap1 _asmy_main_save_game true)
            (SaveGame|SaveGametoSlot _asmy_main_save_game "MainSave" :!label _label)
            (Audio|PlaySoundatLocation "/Game/Game/Sound_Logic/Sounds/ActivateEndMir.ActivateEndMir" (Transformation|GetWorldLocation (Variables|Default|GetLever)) "0, 0, 0" 1.0 1.0 0.0 0 0 0 0))
          (:2
            (Variables|/Script/MyFPS.MyMainSaveGame|SetCompleteMap2 _asmy_main_save_game true)
            (goto _label))
          (:3
            (Variables|/Script/MyFPS.MyMainSaveGame|SetCompleteMap3 _asmy_main_save_game true)
            (goto _label)))))))

(fn ConstructionScript)