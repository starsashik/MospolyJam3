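; A crumbling platform that disappears some time after the player character steps on it, then reappears after a restore delay.
; A box overlap with MainCharacterBP sets a Crash flag, so the countdown continues even if the player leaves.
; Tick runs one shared timer for both phases, toggling mesh visibility and collision as Condition flips.
; A DoOnce starts the audio once during the countdown, and each state change stops it.
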(event OnComponentBeginOverlap(Box)
  (params (OverlappedComponent :type Primitive%20Component%20Object%20Reference) (OtherActor :type Actor%20Object%20Reference) (OtherComp :type Primitive%20Component%20Object%20Reference) (OtherBodyIndex :type Integer) (bFromSweep :type Boolean) (SweepResult :type Hit%20Result%20Structure%20%28by%20ref%29))
  (if (Variables|Default|GetCondition)
    (Utilities|Casting|CastToMainCharacterBP OtherActor)
    (Variables|Default|Setplayer true)
    (Variables|Default|SetCrash true)))

(event OnComponentEndOverlap(Box)
  (params (OverlappedComponent :type Primitive%20Component%20Object%20Reference) (OtherActor :type Actor%20Object%20Reference) (OtherComp :type Primitive%20Component%20Object%20Reference) (OtherBodyIndex :type Integer))
  (if (Variables|Default|GetCondition)
    (Utilities|Casting|CastToMainCharacterBP OtherActor)
    (Variables|Default|Setplayer false)))

(event EventTick
  (params (DeltaSeconds :type Float%20%28single-precision%29))
  (bind _staticmesh (Variables|Default|GetStaticMesh))
  (bind _staticmesh_2 (Variables|Default|GetStaticMesh))
  (if (not (Variables|Default|GetCondition))
    (bind _output_get (Variables|Default|Settime (+ (Variables|Default|Gettime) DeltaSeconds)))
    (if (>= _output_get (Variables|Default|GetTimeToRestor))
      (Variables|Default|SetCondition true)
      (Variables|Default|Settime 0.0)
      (Rendering|SetVisibility _staticmesh_2 true false)
      (Collision|SetCollisionEnabled _staticmesh_2 "QueryAndPhysics")
      (Audio|Components|Audio|Stop (Variables|Default|GetAudio) :!label _label)
      (Variables|Default|SetCrash false)
      (goto _label_2 Reset))
    (else
      (if (Variables|Default|Getplayer)
        _
        (elif (Variables|Default|GetCrash)
          _
          (else
            (Variables|Default|Settime 0.0)
            (Audio|Components|Audio|Stop (Variables|Default|GetAudio))
            (goto _label_2 Reset))))
      (bind _output_get_2 (Variables|Default|Settime (+ (Variables|Default|Gettime) DeltaSeconds)))
      (if (>= _output_get_2 (Variables|Default|GetTimeToCrash))
        (Variables|Default|SetCondition false)
        (Variables|Default|Settime 0.0)
        (Rendering|SetVisibility _staticmesh false false)
        (Collision|SetCollisionEnabled _staticmesh "NoCollision")
        (Variables|Default|Setplayer false)
        (goto _label)
        (else
          (Utilities|FlowControl|DoOnce false :!label _label_2
            (:Completed
              (Audio|Components|Audio|Play (Variables|Default|GetAudio) 0.0))))))))

(fn ConstructionScript)