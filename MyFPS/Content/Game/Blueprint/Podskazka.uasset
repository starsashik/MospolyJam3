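; Hint actor (podskazka) that shows its widget component only while the player is near its static mesh.
; On BeginPlay it casts the widget to UI_podskazka, passes itself in as Podsk, and starts a fast looping timer.
; Each timer tick toggles widget visibility by the distance between the mesh and the first player's pawn, avoiding Event Tick.
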(event Custom|ShowWidget
  (bind _returnvalue (Game|Player|GetPlayerPawn 0))
  (Utilities|IsValid _returnvalue
    (:Is%20Valid
      (if (< (Math|Vector|Distance(Vector) (Transformation|GetWorldLocation (Variables|Default|GetStaticMesh)) (Transformation|GetActorLocation _returnvalue)) 4e+02)
        (Rendering|SetVisibility (Variables|Default|GetWidget) true false)
        (else
          (Rendering|SetVisibility (Variables|Default|GetWidget) false false))))))

(event EventBeginPlay
  (bind _asui_podskazka (Utilities|Casting|CastToUI_podskazka (UserInterface|GetWidget (Variables|Default|GetWidget))))
  (Variables|/Game/Game/HUD/UI_podskazka.UI_podskazka_C|SetPodsk _asui_podskazka self)
  (Utilities|Time|SetTimerbyEvent (delegate Custom|ShowWidget) 0.1 true))

(fn ConstructionScript)