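; MainPlayerControllerBP is the player controller that sets up the pause menu and per-level music when play begins.
; On BeginPlay it caches the main character, creates the UI_Pause widget, switches input to game only and stops the current music through ROPGameInstance.
; After a short delay it picks a music cue by current level name and hands it to the game instance.
; The Pause input calls the menu's CustomPause.
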(event EventBeginPlay
  (bind _asmain_character_bp (Utilities|Casting|CastToMainCharacterBP (Game|Player|GetPlayerPawn 0)))
  (Variables|Default|SetAs%20Main%20Character%20BP _asmain_character_bp)
  (Utilities|IsValid (Variables|Default|GetMenuPause)
    (:Is%20Valid
      _)
    (:Is%20Not%20Valid
      (bind _returnvalue (UserInterface|CreateWidget "/Game/Game/Menu/UI_Pause.UI_Pause_C"))
      (Variables|Default|SetMenuPause _returnvalue)))
  (Input|SetInputModeGameOnly self false)
  (bind _asropgame_instance (Utilities|Casting|CastToROPGameInstance (Game|GetGameInstance)))
  (Default|StopMyMusic _asropgame_instance)
  (Utilities|FlowControl|Delay 2.0)
  (bind _returnvalue_2 (Game|GetCurrentLevelName true))
  (switch string _returnvalue_2
    (:FirstPersonMap
      (Default|SetMyMusic _asropgame_instance "/Game/Game/Sound_Logic/Music/Game_Cue.Game_Cue"))
    (:Mir1
      (Default|SetMyMusic _asropgame_instance "/Game/Game/Sound_Logic/Music/Map1_Cue.Map1_Cue"))
    (:Mir2
      (Default|SetMyMusic _asropgame_instance "/Game/Game/Sound_Logic/Music/Map2_Cue.Map2_Cue"))
    (:Mir3
      (Default|SetMyMusic _asropgame_instance "/Game/Game/Sound_Logic/Music/Map3_Cue.Map3_Cue"))))

(event Input|ActionEvents|InputActionPause
  (params (Key :type Key%20Structure :default "None"))
  (:Pressed
    (Default|CustomPause (Variables|Default|GetMenuPause))))

(fn ConstructionScript)